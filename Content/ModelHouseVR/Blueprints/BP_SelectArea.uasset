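; BP_SelectArea is a selectable area in the VR model house that acts as a step in a sequence.
; Its Box collision accepts queries only from step start until the step ends or play stops.
; Overlap toggles a highlight decal and the assigned Guide's popup, printing an error if Guide is unset.
; Selection either fades the camera out and opens the named level, or ends the step when no level is set.
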(event EventOnBeginOverlap
  (bind _guide (Variables|Default|GetGuide))
  (Rendering|SetVisibility (Variables|Default|GetDecal) true false)
  (Utilities|IsValid _guide
    (:Is%20Valid
      (Default|ShowPopup _guide))
    (:Is%20Not%20Valid
      (Development|PrintString "Guide 변수에 선택을 하지 않았습니다 확인하세요" true true "(R=1.000000,G=0.000000,B=0.000000,A=1.000000)" 6e+01))))

(event EventOnEndOverlap
  (bind _guide (Variables|Default|GetGuide))
  (Rendering|SetVisibility (Variables|Default|GetDecal) false false)
  (Utilities|IsValid _guide
    (:Is%20Valid
      (Default|HidePopup _guide))
    (:Is%20Not%20Valid
      (Development|PrintString "Guide 변수에 선택을 하지 않았습니다 확인하세요" true true "(R=1.000000,G=0.000000,B=0.000000,A=1.000000)" 6e+01))))

(event EventOnSelect
  (bind _level_name (Variables|Default|GetLevel%20Name))
  (if (Utilities|Name|NotEqual(Name) _level_name "None")
    (CameraFades|StartCameraFade :self (Game|GetPlayerCameraManager 0) :ToAlpha 1.0 :Duration 3.0)
    (Utilities|FlowControl|Delay 3.0)
    (Game|OpenLevel(byName) _level_name)
    (else
      (CallFunction|OnEndStep))))

(event EventBeginPlay
  (|CallParentFunction)
  (Collision|SetCollisionEnabled (Variables|Default|GetBox) "NoCollision"))

(fn ConstructionScript)

(fn OnStartStep
  (|CallParentFunction)
  (Collision|SetCollisionEnabled (Variables|Default|GetBox) "QueryOnly"))

(fn OnStopPlay
  (|CallParentFunction)
  (Collision|SetCollisionEnabled (Variables|Default|GetBox) "NoCollision"))

(fn OnEndStep
  (|CallParentFunction)
  (Collision|SetCollisionEnabled (Variables|Default|GetBox) "NoCollision"))