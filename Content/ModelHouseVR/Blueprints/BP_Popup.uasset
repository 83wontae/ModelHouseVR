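; BP_Popup is a popup for the ModelHouseVR project that presents a title and description through a widget component.
; On BeginPlay, InitPopup casts the component's user widget to PopupWidget, caches it, fills it from the StrTitle and StrDesc variables and collapses it.
; ShowPopup makes the cached widget visible when called; the Blueprint has no matching hide function.
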(event EventBeginPlay
  (CallFunction|InitPopup))

(fn ConstructionScript)

(fn InitPopup
  (bind _aspopup_widget (Utilities|Casting|CastToPopupWidget (UserInterface|GetUserWidgetObject (Variables|Default|GetWidget))))
  (bind _output_get (Variables|Default|SetPopupWidget _aspopup_widget))
  (Default|SetPopup _output_get (Variables|Default|GetStr%20Title) (Variables|Default|GetStr%20Desc))
  (Widget|SetVisibility (Variables|Default|GetPopupWidget) "Collapsed"))

(fn ShowPopup
  (Widget|SetVisibility (Variables|Default|GetPopupWidget) "Visible"))