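; BP_StepActor is a base actor for one step of the ModelHouseVR step sequence, showing its comment on a text render in the editor.
; On BeginPlay it binds to the game state's change-step dispatcher, starting when the current step matches its own and otherwise calling an empty stop function.
; Start only prints a debug message, while ending asks MHGameMode to switch to its configured next step, if set.
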(event EventBeginPlay
  (CallFunction|InitBind))

(fn ConstructionScript
  (Rendering|Components|TextRender|SetText (Variables|Default|GetTextRender) (Variables|Default|GetComment)))

(fn InitBind
  (bind _asbp_mhgame_state (Utilities|Casting|CastToBP_MHGameState (Game|GetGameState)))
  (EventDispatchers|BindEventtoEventDispatcherChangeStep _asbp_mhgame_state (EventDispatchers|CreateEvent :!event EventChangeState)))

(fn EventChangeState
  (params (CurStep :type EN_ContentStep%20Enum :default "NewEnumerator0"))
  (if (Utilities|Enum|Equal(Enum) CurStep (Variables|Default|GetMyStep))
    (CallFunction|OnStartStep)
    (else
      (CallFunction|OnStopPlay))))

(fn OnStartStep
  (Development|PrintString (Utilities|String|Append "OnStartStep - " (Utilities|GetDisplayName self)) true true "(R=0.000000,G=0.660000,B=1.000000,A=1.000000)" 2e+01))

(fn OnEndStep
  (if (Utilities|Enum|NotEqual(Enum) (Variables|Default|GetNextStep) "NewEnumerator0")
    (bind _asmhgame_mode (Utilities|Casting|CastToMHGameMode (Game|GetGameMode)))
    (Default|DoChangeStep _asmhgame_mode (Variables|Default|GetNextStep))))

(fn OnStopPlay)