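; VR furniture placement actor that previews a piece at the end of a laser and spawns BP_Furniture at that transform on right trigger.
; Each tick, a WorldStatic line trace from the WidgetInteraction component positions the preview mesh and feeds the Niagara laser's endpoints.
; Right-hand axes adjust the clamped laser length and preview yaw.
; A button cycles DT_Furniture meshes, overriding their materials with glass; the selected index passes to the spawned actor.
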(event EventBeginPlay
  (Transformation|SetWorldRotation (Variables|Default|GetStaticMesh) "0, 0, 0" false false)
  (Input|EnableInput (Game|GetPlayerController 0)))

(event Collision|EventActorBeginOverlap
  (params (OtherActor :type Actor%20Object%20Reference)))

(event EventTick
  (params (DeltaSeconds :type Float%20%28single-precision%29))
  (bind _menulaser (Variables|Default|GetMenuLaser))
  (bind _lasercur (Variables|Default|GetLaserCur))
  (bind _menulaser_2 (Variables|Default|GetMenuLaser))
  (bind _widgetinteraction (Variables|Default|GetWidgetInteraction))
  (bind _widgetinteraction_2 (Variables|Default|GetWidgetInteraction))
  (bind _returnvalue (Transformation|GetWorldLocation _widgetinteraction_2))
  (bind _returnvalue_2 (Math|Vector|GetForwardVector _widgetinteraction_2))
  (bind _returnvalue_3 (Transformation|GetWorldLocation _widgetinteraction))
  (bind _returnvalue_4 (* _returnvalue_2 _lasercur))
  (bind _returnvalue_5 (+ _returnvalue _returnvalue_4))
  (bind (_outhit _returnvalue_6) (Collision|LineTraceForObjects _returnvalue_3 (+ _returnvalue_3 (* (Math|Vector|GetForwardVector _widgetinteraction) (Variables|Default|GetLaserCur))) (Utilities|Array|MakeArray "ObjectTypeQuery1") false 0 "None"))
  (if _returnvalue_6
    (Class|NiagaraDataInterfaceArrayFunctionLibrary|SetNiagaraArrayVectorValue _menulaser_2 "User.PointArray" 0 (Transformation|GetWorldLocation (Variables|Default|GetWidgetInteraction)) false) ; MenuLaser start location
    (Class|NiagaraDataInterfaceArrayFunctionLibrary|SetNiagaraArrayVectorValue _menulaser_2 "User.PointArray" 1 (.ImpactPoint (Collision|BreakHitResult _outhit)) false) ; MenuLaser end location
    (Transformation|SetWorldLocation (Variables|Default|GetStaticMesh) (.ImpactPoint (Collision|BreakHitResult _outhit)) false false)
    (else
      (Class|NiagaraDataInterfaceArrayFunctionLibrary|SetNiagaraArrayVectorValue _menulaser "User.PointArray" 0 _returnvalue false) ; MenuLaser start location
      (Class|NiagaraDataInterfaceArrayFunctionLibrary|SetNiagaraArrayVectorValue _menulaser "User.PointArray" 1 _returnvalue_5 false) ; MenuLaser end location
      (Transformation|SetWorldLocation (Variables|Default|GetStaticMesh) _returnvalue_5 false false))))

(event Input|ActionEvents|InputActionTriggerRight
  (params (Key :type Key%20Structure :default "None"))
  (:Pressed
    (Game|SpawnActorfromClass "/Game/ModelHouseVR/Blueprints/BP_Furniture.BP_Furniture_C" (Transformation|GetWorldTransform (Variables|Default|GetStaticMesh)) "Undefined" 0 (Variables|Default|GetIndex) 0)))

(event Input|ActionEvents|InputActionOculusFurniture_Right
  (params (Key :type Key%20Structure :default "None"))
  (:Pressed
    (CallFunction|ChangeFurniture)))

(event Input|AxisEvents|InputAxisMovementAxisRight_X
  (params (AxisValue :type Float%20%28single-precision%29))
  (Transformation|AddWorldRotation (Variables|Default|GetStaticMesh) (Math|Rotator|MakeRotator 0.0 0.0 AxisValue) false false))

(event Input|AxisEvents|InputAxisMovementAxisRight_Y
  (params (AxisValue :type Float%20%28single-precision%29))
  (CallFunction|IncLaser AxisValue))

(fn ConstructionScript)

(fn ChangeFurniture
  (bind _staticmesh (Variables|Default|GetStaticMesh))
  (Math|Integer|IncrementInt (Variables|Default|GetIndex)
    (:%20%20
      (bind _outrownames (DataTable|GetDataTableRowNames "/Game/ModelHouseVR/Data/DT_Furniture.DT_Furniture"))
      (if (<= (Utilities|Array|Length _outrownames) (Variables|Default|GetIndex))
        (Variables|Default|SetIndex 0))
      (bind _returnvalue (Utilities|GetDataTableRow "/Game/ModelHouseVR/Data/DT_Furniture.DT_Furniture" (Utilities|Array|Get(acopy) _outrownames (Variables|Default|GetIndex)))
        (:then
          (bind _returnvalue_2 (Components|StaticMesh|SetStaticMesh (Variables|Default|GetStaticMesh) (Utilities|Struct|BreakST_Furniture _returnvalue)))
          (if _returnvalue_2
            (for _index (range 0 (- (Rendering|Material|GetNumMaterials _staticmesh) 1))
              (Rendering|Material|SetMaterial _staticmesh _index "/Game/EF_FirstFloor/Common/Materials/Glass/WM_GlassDirty_a_Mat.WM_GlassDirty_a_Mat"))))))))

(fn IncLaser
  (params (IncDelta :type Float%20%28single-precision%29))
  (Variables|Default|SetLaserCur (Math|Float|Clamp(Float) (+ (Variables|Default|GetLaserCur) (* IncDelta 1e+01)) 0.0 (Variables|Default|GetLaserMax))))